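; BP_RealPlayer is the player pawn for the "real" layer, which can look around, hide, and raise or lower an in-game game screen.
; It swaps Enhanced Input mapping contexts as the game goes up or down, trading free real-world controls for mini-game controls unless hiding keeps free controls off.
; Mini-game move, cannon, shoot and reload inputs forward to the MiniMGR's player pawn.
; It also shows a fade-in widget and lights a point light while the screen is on.
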(event Input|EnhancedActionEvents|EnhancedInputActionIA_Mini_MoveX
  (params (ActionValue :type Float%20%28double-precision%29) (ElapsedSeconds :type Float%20%28double-precision%29) (TriggeredSeconds :type Float%20%28double-precision%29) (InputAction :type Input%20Action%20Object%20Reference :default "/Game/BP/Mini/Input/IA_Mini_MoveX.IA_Mini_MoveX"))
  (:Triggered
    (Class|MiniPlayer|InputXMove (Variables|/Script/Angelscript.MiniGameManager|GetPlayerPawn (Variables|/Script/Angelscript.MainGameGM|GetMiniMGR (Class|ModuleMainGameGMStatics|GetGMMain))) ActionValue :!label _label))
  (:Started
    (goto _label))
  (:Ongoing
    (goto _label))
  (:Canceled
    (goto _label))
  (:Completed
    (goto _label)))

(event Input|EnhancedActionEvents|EnhancedInputActionIA_Mini_TurnCannonLeft
  (params (ActionValue :type Boolean) (ElapsedSeconds :type Float%20%28double-precision%29) (TriggeredSeconds :type Float%20%28double-precision%29) (InputAction :type Input%20Action%20Object%20Reference :default "/Game/BP/Mini/Input/IA_Mini_TurnCannonLeft.IA_Mini_TurnCannonLeft"))
  (Class|MiniPlayer|TurnCannonLeft (Variables|/Script/Angelscript.MiniGameManager|GetPlayerPawn (Variables|/Script/Angelscript.MainGameGM|GetMiniMGR (Class|ModuleMainGameGMStatics|GetGMMain)))))

(event Input|EnhancedActionEvents|EnhancedInputActionIA_Mini_TurnCannonRight
  (params (ActionValue :type Boolean) (ElapsedSeconds :type Float%20%28double-precision%29) (TriggeredSeconds :type Float%20%28double-precision%29) (InputAction :type Input%20Action%20Object%20Reference :default "/Game/BP/Mini/Input/IA_Mini_TurnCannonRight.IA_Mini_TurnCannonRight"))
  (Class|MiniPlayer|TurnCannonRight (Variables|/Script/Angelscript.MiniGameManager|GetPlayerPawn (Variables|/Script/Angelscript.MainGameGM|GetMiniMGR (Class|ModuleMainGameGMStatics|GetGMMain)))))

(event Input|EnhancedActionEvents|EnhancedInputActionIA_Mini_Shoot
  (params (ActionValue :type Boolean) (ElapsedSeconds :type Float%20%28double-precision%29) (TriggeredSeconds :type Float%20%28double-precision%29) (InputAction :type Input%20Action%20Object%20Reference :default "/Game/BP/Mini/Input/IA_Mini_Shoot.IA_Mini_Shoot"))
  (Class|MiniPlayer|InputShoot (Variables|/Script/Angelscript.MiniGameManager|GetPlayerPawn (Variables|/Script/Angelscript.MainGameGM|GetMiniMGR (Class|ModuleMainGameGMStatics|GetGMMain)))))

(event Input|EnhancedActionEvents|EnhancedInputActionIA_Mini_Reload
  (params (ActionValue :type Boolean) (ElapsedSeconds :type Float%20%28double-precision%29) (TriggeredSeconds :type Float%20%28double-precision%29) (InputAction :type Input%20Action%20Object%20Reference :default "/Game/BP/Mini/Input/IA_Mini_Reload.IA_Mini_Reload"))
  (Class|MiniPlayer|Reload (Variables|/Script/Angelscript.MiniGameManager|GetPlayerPawn (Variables|/Script/Angelscript.MainGameGM|GetMiniMGR (Class|ModuleMainGameGMStatics|GetGMMain)))))

(event Input|EnhancedActionEvents|EnhancedInputActionIA_Real_Hide
  (params (ActionValue :type Boolean) (ElapsedSeconds :type Float%20%28double-precision%29) (TriggeredSeconds :type Float%20%28double-precision%29) (InputAction :type Input%20Action%20Object%20Reference :default "/Game/BP/Real/Player/Input/IA_Real_Hide.IA_Real_Hide"))
  (:Triggered
    (Class|RealPlayer|UnHide))
  (:Ongoing
    (if (not (Variables|Default|GetbHiding))
      (Class|RealPlayer|Hide))))

(event Input|EnhancedActionEvents|EnhancedInputActionIA_Real_GameUpDown
  (params (ActionValue :type Boolean) (ElapsedSeconds :type Float%20%28double-precision%29) (TriggeredSeconds :type Float%20%28double-precision%29) (InputAction :type Input%20Action%20Object%20Reference :default "/Game/BP/Real/Player/Input/IA_Real_GameUpDown.IA_Real_GameUpDown"))
  (Class|RealPlayer|ToggleGameUpDown))

(event Input|EnhancedActionEvents|EnhancedInputActionIA_Real_Look
  (params (ActionValue :type Vector%202D%20Structure) (ElapsedSeconds :type Float%20%28double-precision%29) (TriggeredSeconds :type Float%20%28double-precision%29) (InputAction :type Input%20Action%20Object%20Reference :default "/Game/BP/Real/Player/Input/IA_Real_Look.IA_Real_Look"))
  (Class|RealPlayer|FreeLook ActionValue))

(event EventBeginPlay
  (|CallParentFunction)
  (bind _returnvalue (UserInterface|CreateWidget "/Game/BP/UI/BPUI_FadeIn.BPUI_FadeIn_C"))
  (UserInterface|Viewport|AddtoViewport _returnvalue 0))

(event Collision|EventActorBeginOverlap
  (params (OtherActor :type Actor%20Object%20Reference)))

(event EventTick
  (params (DeltaSeconds :type Float%20%28single-precision%29))
  (|CallParentFunction DeltaSeconds)
  (Rendering|SetVisibility (Variables|Default|GetPointLight) (Variables|Default|GetbScreenOn) false))

(event EventPossessed
  (params (NewController :type Controller%20Object%20Reference))
  (bind _asplayer_controller (Utilities|Casting|CastToPlayerController NewController))
  (Input|AddMappingContext (PlayerController|LocalPlayerSubsystems|GetEnhancedInputLocalPlayerSubsystem _asplayer_controller) "/Game/BP/Real/Player/Input/IMC_RealAlways.IMC_RealAlways" 0 "(bIgnoreAllPressedKeysUntilRelease=True,bForceImmediately=False,bNotifyUserSettings=False)"))

(event EventGameDoneUp
  (|CallParentFunction)
  (Input|AddMappingContext (PlayerController|LocalPlayerSubsystems|GetEnhancedInputLocalPlayerSubsystem (Game|GetPlayerController 0)) "/Game/BP/Mini/Input/IMC_Mini.IMC_Mini" 0 "(bIgnoreAllPressedKeysUntilRelease=True,bForceImmediately=False,bNotifyUserSettings=False)"))

(event EventGameUp
  (|CallParentFunction)
  (if (not (Variables|Default|GetbHiding))
    (Input|RemoveMappingContext (PlayerController|LocalPlayerSubsystems|GetEnhancedInputLocalPlayerSubsystem (Game|GetPlayerController 0)) "/Game/BP/Real/Player/Input/IMC_RealFree.IMC_RealFree" "(bIgnoreAllPressedKeysUntilRelease=True,bForceImmediately=False,bNotifyUserSettings=False)")
    (Development|PrintString "input up")))

(event EventGameDown
  (bind _returnvalue (Game|GetPlayerController 0))
  (bind _returnvalue_2 (PlayerController|LocalPlayerSubsystems|GetEnhancedInputLocalPlayerSubsystem _returnvalue))
  (|CallParentFunction)
  (Input|RemoveMappingContext _returnvalue_2 "/Game/BP/Mini/Input/IMC_Mini.IMC_Mini" "(bIgnoreAllPressedKeysUntilRelease=True,bForceImmediately=False,bNotifyUserSettings=False)")
  (if (not (Variables|Default|GetbHiding))
    (Input|AddMappingContext _returnvalue_2 "/Game/BP/Real/Player/Input/IMC_RealFree.IMC_RealFree" 0 "(bIgnoreAllPressedKeysUntilRelease=True,bForceImmediately=False,bNotifyUserSettings=False)")))

(fn ConstructionScript
  (|CallParentFunction))