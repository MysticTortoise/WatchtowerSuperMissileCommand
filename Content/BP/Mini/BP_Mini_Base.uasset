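; BP_Mini_Base is a child base actor whose destruction can trigger game over.
; Its DestroyBase event runs the parent logic, then queries the bases still alive.
; When none remain, it stores the death texture on the game instance and opens the MAP_GameOver level.
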(event EventBeginPlay
  (|CallParentFunction) ; This node is disabled and will not be called.\nDrag off pins to build functionality.
)

(event Collision|EventActorBeginOverlap
  (params (OtherActor :type Actor%20Object%20Reference)))

(event EventTick
  (params (DeltaSeconds :type Float%20%28single-precision%29)))

(event EventDestroyBase
  (|CallParentFunction)
  (bind _returnvalue (Class|ModuleMinigameMiniBaseStatics|GetAliveBases))
  (if (Utilities|Array|IsEmpty _returnvalue)
    (Variables|/Script/Angelscript.HideGameInstance|SetGOTexture (Class|ModuleGameInstanceStatics|GetGI) "/Game/Textures/ui/TEX_GameDeath.TEX_GameDeath")
    (Game|OpenLevel(byName) "MAP_GameOver")))

(fn ConstructionScript
  (|CallParentFunction))