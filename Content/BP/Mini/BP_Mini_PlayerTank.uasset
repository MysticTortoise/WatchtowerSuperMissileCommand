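; BP_Mini_PlayerTank is the player-controlled tank, apparently for a minigame, acting as a thin input layer over inherited logic.
; Enhanced Input actions for horizontal movement, cannon rotation, shooting and reloading each forward to a matching function that is not defined here.
; The move axis passes its value on in every trigger phase, including completion and cancellation.
; BeginPlay and construction just call the parent, and Tick is disabled.
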(event Input|EnhancedActionEvents|EnhancedInputActionIA_Mini_MoveX
  (params (ActionValue :type Float%20%28double-precision%29) (ElapsedSeconds :type Float%20%28double-precision%29) (TriggeredSeconds :type Float%20%28double-precision%29) (InputAction :type Input%20Action%20Object%20Reference :default "/Game/BP/Mini/Input/IA_Mini_MoveX.IA_Mini_MoveX"))
  (:Triggered
    (Class|MiniPlayer|InputXMove ActionValue :!label _label))
  (:Started
    (goto _label))
  (:Ongoing
    (goto _label))
  (:Canceled
    (goto _label))
  (:Completed
    (goto _label)))

(event Input|EnhancedActionEvents|EnhancedInputActionIA_Mini_TurnCannonLeft
  (params (ActionValue :type Boolean) (ElapsedSeconds :type Float%20%28double-precision%29) (TriggeredSeconds :type Float%20%28double-precision%29) (InputAction :type Input%20Action%20Object%20Reference :default "/Game/BP/Mini/Input/IA_Mini_TurnCannonLeft.IA_Mini_TurnCannonLeft"))
  (Class|MiniPlayer|TurnCannonLeft))

(event Input|EnhancedActionEvents|EnhancedInputActionIA_Mini_TurnCannonRight
  (params (ActionValue :type Boolean) (ElapsedSeconds :type Float%20%28double-precision%29) (TriggeredSeconds :type Float%20%28double-precision%29) (InputAction :type Input%20Action%20Object%20Reference :default "/Game/BP/Mini/Input/IA_Mini_TurnCannonRight.IA_Mini_TurnCannonRight"))
  (Class|MiniPlayer|TurnCannonRight))

(event Input|EnhancedActionEvents|EnhancedInputActionIA_Mini_Shoot
  (params (ActionValue :type Boolean) (ElapsedSeconds :type Float%20%28double-precision%29) (TriggeredSeconds :type Float%20%28double-precision%29) (InputAction :type Input%20Action%20Object%20Reference :default "/Game/BP/Mini/Input/IA_Mini_Shoot.IA_Mini_Shoot"))
  (Class|MiniPlayer|InputShoot))

(event Input|EnhancedActionEvents|EnhancedInputActionIA_Mini_Reload
  (params (ActionValue :type Boolean) (ElapsedSeconds :type Float%20%28double-precision%29) (TriggeredSeconds :type Float%20%28double-precision%29) (InputAction :type Input%20Action%20Object%20Reference :default "/Game/BP/Mini/Input/IA_Mini_Reload.IA_Mini_Reload"))
  (Class|MiniPlayer|Reload))

(event EventBeginPlay
  (|CallParentFunction))

(event Collision|EventActorBeginOverlap
  (params (OtherActor :type Actor%20Object%20Reference)))

(event EventTick
  (params (DeltaSeconds :type Float%20%28single-precision%29))
  (|CallParentFunction DeltaSeconds) ; This node is disabled and will not be called.\nDrag off pins to build functionality.
)

(fn ConstructionScript
  (|CallParentFunction))